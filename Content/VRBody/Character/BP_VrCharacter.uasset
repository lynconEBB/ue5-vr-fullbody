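; VR player character Blueprint that provides thumbstick-driven sliding locomotion from either motion controller.
; BeginPlay adds the Enhanced Input mapping context, and both controller movement actions feed a shared handler that selects that hand's axes.
; A helper converts the axes into yaw, clamped magnitude and a deadzone check.
; Valid input rotates the VR forward vector for AddMovementInput; otherwise the forward vector is used unrotated.
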(event Input|EnhancedActionEvents|EnhancedInputActionIA_RightControllerMovement
  (params (ActionValue :type Float%20%28double-precision%29) (ElapsedSeconds :type Float%20%28double-precision%29) (TriggeredSeconds :type Float%20%28double-precision%29) (InputAction :type Input%20Action%20Object%20Reference :default "/Game/VRBody/Input/IA_RightControllerMovement.IA_RightControllerMovement"))
  (CallFunction|HandleSlidingMovement (Variables|Default|GetRightMotionController)))

(event Input|EnhancedActionEvents|EnhancedInputActionIA_LeftControllerMovement
  (params (ActionValue :type Float%20%28double-precision%29) (ElapsedSeconds :type Float%20%28double-precision%29) (TriggeredSeconds :type Float%20%28double-precision%29) (InputAction :type Input%20Action%20Object%20Reference :default "/Game/VRBody/Input/IA_LeftControllerMovement.IA_LeftControllerMovement"))
  (CallFunction|HandleSlidingMovement (Variables|Default|GetLeftMotionController)))

(event EventBeginPlay
  (bind _asplayer_controller (Utilities|Casting|CastToPlayerController (Pawn|GetController)))
  (Input|AddMappingContext (PlayerController|LocalPlayerSubsystems|GetEnhancedInputLocalPlayerSubsystem _asplayer_controller) "/Game/VRBody/Input/IMC_VRMovement.IMC_VRMovement" 0 "(bIgnoreAllPressedKeysUntilRelease=True,bForceImmediately=False,bNotifyUserSettings=False)"))

(fn ConstructionScript)

(fn HandleSlidingMovement
  (params (CallingHand :type Grip%20Motion%20Controller%20Component%20Object%20Reference))
  (switch Utilities|FlowControl|Switch|SwitchonEControllerHand (Class|GripMotionControllerComponent|GetHandType CallingHand)
    (:Left
      ;[1 1 1] Get correct hand axis values
      (LocalVariables|SetThumbY (Input|EnhancedActionValues|GetIA_LeftDpadY))
      (LocalVariables|SetThumbX (Input|EnhancedActionValues|GetIA_LeftDpadX)))
    (:Right
      (LocalVariables|SetThumbY (Input|EnhancedActionValues|GetIA_RightDpadY))
      (LocalVariables|SetThumbX (Input|EnhancedActionValues|GetIA_RightDpadX))))
  (Development|PrintString (Utilities|String|ToString(Float) (LocalVariables|GetThumbY)))
  (if (.WasValid (CallFunction|CalcPadRotationandMagnitude (LocalVariables|GetThumbY) (LocalVariables|GetThumbX) (Variables|Default|GetDPadVelocityScaler) (Variables|Default|GetSlidingMovementDeadZone)))
    (LocalVariables|SetDirection (Math|Vector|RotateVector (Class|VRBaseCharacter|GetVRForwardVector) (.Rotation (CallFunction|CalcPadRotationandMagnitude (LocalVariables|GetThumbY) (LocalVariables|GetThumbX) (Variables|Default|GetDPadVelocityScaler) (Variables|Default|GetSlidingMovementDeadZone)))))
    (else
      (LocalVariables|SetDirection (Class|VRBaseCharacter|GetVRForwardVector))))
  (Pawn|Input|AddMovementInput (LocalVariables|GetDirection) (.Magnitude (CallFunction|CalcPadRotationandMagnitude (LocalVariables|GetThumbY) (LocalVariables|GetThumbX) (Variables|Default|GetDPadVelocityScaler) (Variables|Default|GetSlidingMovementDeadZone))) false))

(fn CalcPadRotationandMagnitude
  (params (YAxis :type Float%20%28double-precision%29) (XAxis :type Float%20%28double-precision%29) (OptMagnitudeScaler :type Float%20%28double-precision%29) (OptionalDeadzone :type Float%20%28double-precision%29))
  (return (Math|Rotator|MakeRotfromX (Math|Vector|MakeVector YAxis XAxis 0.0)) (Math|Float|Clamp(Float) (Math|Vector|GetMaxElement (Math|Vector|MakeVector (Math|Float|Absolute(Float) (* YAxis OptMagnitudeScaler)) (Math|Float|Absolute(Float) (* XAxis OptMagnitudeScaler)) 0.0))) (> (+ (Math|Float|Absolute(Float) YAxis) (Math|Float|Absolute(Float) XAxis)) OptionalDeadzone)))